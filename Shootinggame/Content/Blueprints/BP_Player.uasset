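; BP_Player is the player actor, which moves on the X/Y plane and fires bullets.
; Each Tick normalizes the horizontal and vertical input into a direction, scales it by MoveSpeed and delta time, and sets the location directly without sweeping.
; Pressing the Fire action spawns a BP_Bullet at the FirePos component's world transform, ignoring collisions.
; The IA_Move event is present but empty.
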(event `self.ReceiveTick`
  (params (DeltaSeconds :type "Float (single-precision)"))
  (`self.K2_SetActorLocation` (+ (`self.K2_GetActorLocation`) (* (* (`KismetMathLibrary.Normal` (`KismetMathLibrary.MakeVector` (`self.GetInputAxisValue`) (`self.GetInputAxisValue`))) (`self.moveSpeed`)) DeltaSeconds))))

(event `InputAction|Fire`
  (params (Key :type "Key Structure"))
  (:`Pressed`
    (`|SpawnActorFromClass` "/Game/Blueprints/BP_Bullet.BP_Bullet_C" (`SceneComponent.K2_GetComponentToWorld` (`self.firePos`)) "AlwaysSpawn" "MultiplyWithRoot" null null)))

(event `EnhancedInput|/Game/InputAction/IA_Move`
  (params (ActionValue :type "Vector Structure") (ElapsedSeconds :type "Float (double-precision)") (TriggeredSeconds :type "Float (double-precision)") (InputAction :type "InputAction Object Reference" :default "/Game/InputAction/IA_Move.IA_Move")))

(fn `UserConstructionScript`)